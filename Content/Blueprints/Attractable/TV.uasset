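; TV is an attractable prop Blueprint that highlights its static mesh when the mouse is over it.
; The mouse-over event swaps material slot 0 to a blue rim material, and the mouse-leave event sets that slot to the building material.
; The BeginPlay, overlap and Tick events are disabled stubs, and the construction script only calls its parent.
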(event EventBeginPlay
  (|CallParentFunction) ; This node is disabled and will not be called.\nDrag off pins to build functionality.
)

(event Collision|EventActorBeginOverlap
  (params (OtherActor :type Actor%20Object%20Reference))
  (|CallParentFunction OtherActor) ; This node is disabled and will not be called.\nDrag off pins to build functionality.
)

(event EventTick
  (params (DeltaSeconds :type Float%20%28single-precision%29))
  (|CallParentFunction DeltaSeconds) ; This node is disabled and will not be called.\nDrag off pins to build functionality.
)

(event EventOnMouseOver
  (Rendering|Material|SetMaterial (Variables|Default|GetStaticMesh) 0 "/Game/Assets/Models/rimblue.rimblue"))

(event EventOnMouseLeave
  (Rendering|Material|SetMaterial (Variables|Default|GetStaticMesh) 0 "/Game/Assets/Materials/MI_Building.MI_Building"))

(fn ConstructionScript
  (|CallParentFunction))
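; Laser pointer actor in the Attractable folder that reacts to mouse hover and clicks.
; Hovering swaps the mesh to a blue rim material and activates the Laser component; leaving restores the material and deactivates it.
; Clicking fires a visibility line trace from the second mesh, but its end is the scaled forward vector without the start location added, and the result is unused.
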(event EventBeginPlay
  (|CallParentFunction) ; This node is disabled and will not be called.\nDrag off pins to build functionality.
)

(event Collision|EventActorBeginOverlap
  (params (OtherActor :type Actor%20Object%20Reference))
  (|CallParentFunction OtherActor) ; This node is disabled and will not be called.\nDrag off pins to build functionality.
)

(event EventTick
  (params (DeltaSeconds :type Float%20%28single-precision%29))
  (|CallParentFunction DeltaSeconds) ; This node is disabled and will not be called.\nDrag off pins to build functionality.
)

(event EventOnMouseOver
  (Rendering|Material|SetMaterial (Variables|Default|GetStaticMesh) 0 "/Game/Assets/Models/rimblue.rimblue")
  (Components|Activation|Activate (Variables|Default|GetLaser) false))

(event EventOnMouseLeave
  (Rendering|Material|SetMaterial (Variables|Default|GetStaticMesh) 0 "/Game/Assets/Models/lambert1.lambert1")
  (Components|Activation|Deactivate (Variables|Default|GetLaser)))

(event MouseInput|EventActorOnClicked
  (params (ButtonPressed :type Key%20Structure :default "None"))
  (bind _staticmesh1 (Variables|Default|GetStaticMesh1))
  (Collision|LineTraceByChannel (Transformation|GetWorldLocation _staticmesh1) (* (Math|Vector|Normalize (Math|Vector|GetForwardVector _staticmesh1)) 2e+03) "TraceTypeQuery1" false 0 "None"))

(fn ConstructionScript
  (|CallParentFunction))
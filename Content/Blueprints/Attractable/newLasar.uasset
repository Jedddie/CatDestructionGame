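; Interactable laser actor that attracts a cat to the point its beam hits.
; Mouse hover swaps the mesh to a blue rim material and activates a particle system; leaving restores the default material and deactivates the particles.
; Interact line-traces from StaticMesh1 along its negative forward vector on the Visibility channel, then passes the impact point and Force to the cat's Attract without checking for a hit.
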(event EventBeginPlay
  (|CallParentFunction) ; This node is disabled and will not be called.\nDrag off pins to build functionality.
)

(event Collision|EventActorBeginOverlap
  (params (OtherActor :type Actor%20Object%20Reference))
  (|CallParentFunction OtherActor) ; This node is disabled and will not be called.\nDrag off pins to build functionality.
)

(event EventTick
  (params (DeltaSeconds :type Float%20%28single-precision%29))
  (|CallParentFunction DeltaSeconds) ; This node is disabled and will not be called.\nDrag off pins to build functionality.
)

(event EventInteract
  (params (Cat :type Cat%20Object%20Reference))
  (bind _staticmesh1 (Variables|Default|GetStaticMesh1))
  (bind _returnvalue (Transformation|GetWorldLocation _staticmesh1))
  (bind _returnvalue_2 (Math|Vector|GetForwardVector _staticmesh1))
  (bind _returnvalue_3 (Math|Vector|Normalize _returnvalue_2))
  (bind _outhit (Collision|LineTraceByChannel (+ _returnvalue (* _returnvalue_3 -1e+01)) (+ _returnvalue (* _returnvalue_3 -2e+03)) "TraceTypeQuery1" false 0 "None"))
  (Default|Attract Cat (.impactpoint _outhit) (Variables|Default|Getforce)))

(event EventOnMouseOver
  (Rendering|Material|SetMaterial (Variables|Default|GetStaticMesh) 0 "/Game/Assets/Models/rimblue.rimblue")
  (Components|Activation|Activate (Variables|Default|GetParticleSystem) false))

(event EventOnMouseLeave
  (Rendering|Material|SetMaterial (Variables|Default|GetStaticMesh) 0 "/Game/Assets/Models/lambert1.lambert1")
  (Components|Activation|Deactivate (Variables|Default|GetParticleSystem)))

(fn ConstructionScript
  (|CallParentFunction))
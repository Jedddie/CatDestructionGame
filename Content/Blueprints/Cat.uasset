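; Cat actor with lives that is pushed around by physics and ends the game when it runs out of lives.
; Attract and Repel events apply a force of given magnitude to the mesh, toward or away from a world location.
; Hits with a normal impulse above the hurt threshold cost a life, and reaching zero opens the EndScreen level.
; Unconnected nodes for partial ragdoll physics below the CatChest bone never run.
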(event Custom|Attract
  (params (World%20Location :type Vector) (Magnitude :type Float%20%28single-precision%29))
  (Physics|AddForce (Variables|Default|GetMesh) (* (Math|Vector|Normalize (- World%20Location (Transformation|GetWorldLocation (Variables|Default|GetMesh)))) Magnitude) "None" false))

(event Custom|Repel
  (params (World%20Location :type Vector) (Magnitude :type Float%20%28single-precision%29))
  (Physics|AddForce (Variables|Default|GetMesh) (* (Math|Vector|Normalize (- (Transformation|GetWorldLocation (Variables|Default|GetMesh)) World%20Location)) Magnitude) "None" false))

(event EventBeginPlay)

(event Collision|EventActorBeginOverlap
  (params (OtherActor :type Actor%20Object%20Reference)))

(event EventTick
  (params (DeltaSeconds :type Float%20%28single-precision%29)))

(event Collision|EventHit
  (params (MyComp :type Primitive%20Component%20Object%20Reference) (Other :type Actor%20Object%20Reference) (OtherComp :type Primitive%20Component%20Object%20Reference) (bSelfMoved :type Boolean) (HitLocation :type Vector :default "0, 0, 0") (HitNormal :type Vector :default "0, 0, 0") (NormalImpulse :type Vector :default "0, 0, 0") (Hit :type Hit%20Result%20Structure%20%28by%20ref%29))
  (if (> (Math|Vector|VectorLength NormalImpulse) (Variables|Default|GetHurtThreshold))
    (bind _result (Math|Integer|DecrementInt (Variables|Default|GetLives))
      (:%20%20
        ;[1 1 1] Close Game Loop
        (if (<= _result 0)
          (Game|OpenLevel(byName) "EndScreen"))))))

(fn ConstructionScript)
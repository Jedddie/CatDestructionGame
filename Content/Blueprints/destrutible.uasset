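; Destructible vase actor that breaks when the Cat hits it hard enough and awards points.
; On Hit, an impulse above DestructionThreshold sets a one-time IsDestroyed flag and applies damage to the VaseDM destructible at the impact point, pushing along the normal impulse with scaled-down strength.
; It then adds ScoreValue to the Score held in CatGameInstance.
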(event EventBeginPlay)

(event Collision|EventActorBeginOverlap
  (params (OtherActor :type Actor%20Object%20Reference)))

(event Collision|EventHit
  (params (MyComp :type Primitive%20Component%20Object%20Reference) (Other :type Actor%20Object%20Reference) (OtherComp :type Primitive%20Component%20Object%20Reference) (bSelfMoved :type Boolean) (HitLocation :type Vector :default "0, 0, 0") (HitNormal :type Vector :default "0, 0, 0") (NormalImpulse :type Vector :default "0, 0, 0") (Hit :type Hit%20Result%20Structure%20%28by%20ref%29))
  (bind _returnvalue (Math|Vector|VectorLength NormalImpulse))
  (Utilities|Casting|CastToCat Other)
  (if (and (> _returnvalue (Variables|Default|GetDestructionThreshold)) (not (Variables|Default|GetisDestroyed)))
    (Variables|Default|SetisDestroyed true)
    (Class|DestructibleComponent|ApplyDamage (Variables|Default|GetVase_DM) 1.0 HitLocation (Math|Vector|Normalize NormalImpulse) (* _returnvalue 0.2))
    (bind _ascat_game_instance (Utilities|Casting|CastToCatGameInstance (Game|GetGameInstance)))
    (Variables|/Game/Blueprints/CatGameInstance.CatGameInstance_C|Setscore _ascat_game_instance (+ (Variables|/Game/Blueprints/CatGameInstance.CatGameInstance_C|Getscore _ascat_game_instance) (Variables|Default|GetScoreValue)))))

(fn ConstructionScript)
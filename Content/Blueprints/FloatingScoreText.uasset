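; FloatingScoreText is an actor that shows a dollar-prefixed score as floating world text, set through SetValue.
; Each tick it samples the RelativeLocation vector curve, scaled by a random per-instance factor, to offset the text from its spawn location.
; It also yaws the text toward the player camera and ramps its alpha up with elapsed time, then destroys itself when the curve ends.
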(event EventBeginPlay
  (Variables|Default|SetInitial%20World%20Location (Transformation|GetWorldLocation (Variables|Default|GetTextRender)))
  (Variables|Default|Setinitial%20time (Utilities|Time|GetTimeSeconds))
  (Variables|Default|Setmovement%20scale (Math|Random|RandomFloatinRange 0.9 1.5)))

(event Collision|EventActorBeginOverlap
  (params (OtherActor :type Actor%20Object%20Reference)))

(event EventTick
  (params (DeltaSeconds :type Float%20%28single-precision%29))
  (bind _returnvalue (Utilities|Time|GetTimeSeconds))
  (bind _relativelocation (Variables|Default|GetRelativeLocation))
  (bind _initial_time (Variables|Default|Getinitial%20time))
  (bind _textrender (Variables|Default|GetTextRender))
  (bind _returnvalue_2 (- _returnvalue _initial_time))
  (bind (_mintime _maxtime) (Math|Curves|GetTimeRange _relativelocation))
  (bind _textrendercolor (Variables|/Script/Engine.TextRenderComponent|GetTextRenderColor _textrender))
  (Transformation|SetWorldLocationAndRotation (Variables|Default|GetTextRender) (+ (Variables|Default|GetInitial%20World%20Location) (* (Math|Curves|GetVectorValue _relativelocation _returnvalue_2) (Variables|Default|Getmovement%20scale))) (Math|Rotator|MakeRotator 0.0 0.0 (.yaw (Math|Rotator|FindLookatRotation (Transformation|GetWorldLocation (Variables|Default|GetTextRender)) (Camera|GetCameraLocation (Variables|/Script/Engine.PlayerController|GetPlayerCameraManager (Game|GetPlayerController 0)))))) false false)
  (Rendering|Components|TextRender|SetTextRenderColor _textrender (Math|Color|MakeColor (.b _textrendercolor) (.g _textrendercolor) (.r _textrendercolor) (Math|Conversions|ToByte(Integer) (Math|Float|Truncate (* 255 (/ _returnvalue_2 (- _maxtime _mintime)))))))
  (if (> _returnvalue_2 _maxtime)
    (Actor|DestroyActor)))

(fn ConstructionScript)

(fn SetValue
  (params (Score%20Value :type Float%20%28single-precision%29))
  (Rendering|Components|TextRender|SetText (Variables|Default|GetTextRender) (Utilities|Text|ToText(String) (Utilities|String|BuildString(Float) "" "$" Score%20Value))))
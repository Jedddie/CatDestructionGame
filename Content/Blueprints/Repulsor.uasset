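; Repulsor is an interactable Blueprint that pushes a cat away when the cat interacts with it.
; Its Interact event calls Repel on the passed-in Cat, supplying the static mesh's world location as the origin and the Force variable as the magnitude.
; The push itself is left to the cat's Repel function, and the Repulsor runs no tick or overlap logic.
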(event EventBeginPlay
  (|CallParentFunction) ; This node is disabled and will not be called.\nDrag off pins to build functionality.
)

(event Collision|EventActorBeginOverlap
  (params (OtherActor :type Actor%20Object%20Reference))
  (|CallParentFunction OtherActor) ; This node is disabled and will not be called.\nDrag off pins to build functionality.
)

(event EventTick
  (params (DeltaSeconds :type Float%20%28single-precision%29))
  (|CallParentFunction DeltaSeconds) ; This node is disabled and will not be called.\nDrag off pins to build functionality.
)

(event EventInteract
  (params (Cat :type Cat%20Object%20Reference))
  (Default|Repel Cat (Transformation|GetWorldLocation (Variables|Default|GetStaticMesh)) (Variables|Default|Getforce)))

(fn ConstructionScript
  (|CallParentFunction))
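; TunaCan is an interactable Blueprint object that a cat can open once.
; On Interact, if the Open flag is false, it plays the can's opening animation without looping, calls the parent Interact with the Cat, then sets Open.
; The flag blocks any later interaction, including the parent's logic, and the other event stubs are disabled.
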(event EventBeginPlay
  (|CallParentFunction) ; This node is disabled and will not be called.\nDrag off pins to build functionality.
)

(event Collision|EventActorBeginOverlap
  (params (OtherActor :type Actor%20Object%20Reference))
  (|CallParentFunction OtherActor) ; This node is disabled and will not be called.\nDrag off pins to build functionality.
)

(event EventTick
  (params (DeltaSeconds :type Float%20%28single-precision%29))
  (|CallParentFunction DeltaSeconds) ; This node is disabled and will not be called.\nDrag off pins to build functionality.
)

(event EventInteract
  (params (Cat :type Cat%20Object%20Reference))
  (if (not (Variables|Default|GetOpen))
    (Components|Animation|PlayAnimation (Variables|Default|GetCan) "/Game/Assets/Models/Interactables/Tuna_Can_Anim.Tuna_Can_Anim" false)
    (|CallParentFunction Cat)
    (Variables|Default|SetOpen true)))

(fn ConstructionScript
  (|CallParentFunction))